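; BP_CCharacter is a character Blueprint with a weapon and a CTrace component.
; On LateBeginPlay it assigns the weapon's mesh to CTrace as its WeaponMesh, while BeginPlay and the construction script are empty.
; A disconnected graph, which never runs, plays draw or sheath montages based on SwordDraw and snaps an attachment to the S_Draw or S_Sheath socket on the montage notify.
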(event `self.ReceiveBeginPlay`)

(event `self.LateBeginPlay`
  (set `CTraceComponent.WeaponMesh` (`CMyWeapon.Weapon` (`self.Weapon`)) (`self.CTrace`)))

(event `EnhancedInput|/Game/Input/Action/IA_Draw`
  (params (ActionValue :type Boolean) (ElapsedSeconds :type "Float (double-precision)") (TriggeredSeconds :type "Float (double-precision)") (InputAction :type "InputAction Object Reference" :default "/Game/Input/Action/IA_Draw.IA_Draw")))

(fn `UserConstructionScript`)