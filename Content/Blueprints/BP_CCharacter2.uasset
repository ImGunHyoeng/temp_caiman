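; BP_CCharacter2 is a character Blueprint that appears to be a test bed for hit reactions.
; GetHit prints a debug message and passes the impact point and offense to the parent implementation.
; Mesh hit and overlap events print bone names, while BeginPlay, AnyDamage and capsule overlap are empty.
; Disconnected nodes hold unused damage binding, physics ragdoll blending and a strong-attack reaction montage.
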(event `self.ReceiveBeginPlay`)

(event `HitInterface.GetHit`
  (params (ImpactPoint :type "Vector Structure (by ref)") (Offense :type "Actor Object Reference"))
  (`KismetSystemLibrary.PrintString` "Hello")
  (`parent.GetHit` ImpactPoint Offense))

(event `self.ReceiveAnyDamage`
  (params (Damage :type "Float (single-precision)") (DamageType :type "DamageType Object Reference") (InstigatedBy :type "Controller Object Reference") (DamageCauser :type "Actor Object Reference"))
  ;[1 1 1] 플레이어 피격처리
)

(event `self.Mesh.OnComponentHit`
  (params (HitComponent :type "PrimitiveComponent Object Reference") (OtherActor :type "Actor Object Reference") (OtherComp :type "PrimitiveComponent Object Reference") (NormalImpulse :type "Vector Structure") (Hit :type "HitResult Structure (by ref)"))
  (`KismetSystemLibrary.PrintString` (`KismetStringLibrary.Conv_NameToString` Hit_BoneName)))

(event `self.Mesh.OnComponentBeginOverlap`
  (params (OverlappedComponent :type "PrimitiveComponent Object Reference") (OtherActor :type "Actor Object Reference") (OtherComp :type "PrimitiveComponent Object Reference") (OtherBodyIndex :type Integer) (bFromSweep :type Boolean) (SweepResult :type "HitResult Structure (by ref)"))
  (`KismetSystemLibrary.PrintString` (`KismetStringLibrary.Conv_NameToString` SweepResult_HitBoneName)))

(event `self.CapsuleComponent.OnComponentBeginOverlap`
  (params (OverlappedComponent :type "PrimitiveComponent Object Reference") (OtherActor :type "Actor Object Reference") (OtherComp :type "PrimitiveComponent Object Reference") (OtherBodyIndex :type Integer) (bFromSweep :type Boolean) (SweepResult :type "HitResult Structure (by ref)")))

(fn `UserConstructionScript`)