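; Enemy character with boss-style close, jump and fireball attacks, controlled through an AI brain component.
; Detect, LAttack and CAttack overlaps track the player's presence and range in flags, with Detect also toggling a widget.
; Custom events play attack montages, while Fire spawns a projectile from FlameSocket, pitched toward the player.
; Point damage sets timed hit and cooldown flags, or triggers Death, which stops AI logic and disables collision and movement.
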(event `self.ReceiveBeginPlay`)

(event `self.ReceivePointDamage`
  (params (Damage :type "Float (single-precision)") (DamageType :type "DamageType Object Reference") (HitLocation :type "Vector Structure") (HitNormal :type "Vector Structure") (HitComponent :type "PrimitiveComponent Object Reference") (BoneName :type Name) (ShotFromDirection :type "Vector Structure") (InstigatedBy :type "Controller Object Reference") (DamageCauser :type "Actor Object Reference") (HitInfo :type "HitResult Structure (by ref)"))
  ;[1 1 1] 맞았을 경우 이벤트 처리
  (set `self.bIsAttacked` true)
  (if (not (`self.bIsLive`))
    (`self.Death`))
  (set `self.bIsCoolTime` true)
  (`KismetSystemLibrary.Delay` 1.5)
  (set `self.bIsAttacked` false)
  (set `self.bIsCoolTime` false))

(event `HitInterface.GetHit`
  (params (ImpactPoint :type "Vector Structure (by ref)") (Offense :type "Actor Object Reference"))
  (`GameplayStatics.PlaySound2D` "/Game/Audio/Metasound/SFX_SwordHit.SFX_SwordHit" 1.0 1.0 0.0 null null)
  (`parent.GetHit` ImpactPoint Offense))

(event `ProjectileBossAnimMontage`
  ;[1 1 1] 구체발사 애님 몽타주
  (`self.PlayAnimMontage` "/Game/Enemy/Anim/AM_flame.AM_flame"))

(event `CloseAttack`
  ;[1 1 1] 근접공격
  (`self.PlayAnimMontage` "/Game/Enemy/Anim/AM_CloseAttack_L.AM_CloseAttack_L"))

(event `self.detect.OnComponentEndOverlap`
  (params (OverlappedComponent :type "PrimitiveComponent Object Reference") (OtherActor :type "Actor Object Reference") (OtherComp :type "PrimitiveComponent Object Reference") (OtherBodyIndex :type Integer))
  ;[1 1 1] 충돌에서 벗어남 처리
  (cast `/Game/Blueprints/BP_CCharacter` OtherActor)
  (`self.SetWidgetVisible` false)
  (set `self.Enemy detected` null)
  (set `self.bIsDetect` false))

(event `self.detect.OnComponentBeginOverlap`
  (params (OverlappedComponent :type "PrimitiveComponent Object Reference") (OtherActor :type "Actor Object Reference") (OtherComp :type "PrimitiveComponent Object Reference") (OtherBodyIndex :type Integer) (bFromSweep :type Boolean) (SweepResult :type "HitResult Structure (by ref)"))
  ;[1 1 1] 충돌시에 적감지 처리
  (bind _asbp_ccharacter (cast `/Game/Blueprints/BP_CCharacter` OtherActor))
  (`self.SetWidgetVisible` true)
  (set `self.Enemy detected` _asbp_ccharacter)
  (set `self.bIsDetect` true))

(event `Fire`
  (bind _returnvalue (`SceneComponent.GetSocketLocation` (`self.Mesh`) "FlameSocket"))
  (bind (_returnvalue_roll _returnvalue_pitch _returnvalue_yaw) (`KismetMathLibrary.BreakRotator` (`SceneComponent.GetSocketRotation` (`self.Mesh`) "FlameSocket")))
  (bind (_returnvalue_roll_2 _returnvalue_pitch_2) (`KismetMathLibrary.BreakRotator` (`KismetMathLibrary.FindLookAtRotation` _returnvalue (`self.K2_GetActorLocation` (`GameplayStatics.GetPlayerPawn` 0)))))
  ;[1 1 1] 발사
  (`GameplayStatics.PlaySound2D` "/Game/Audio/Metasound/SFX_FIreball.SFX_FIreball" 1.0 1.0 0.0 null null)
  (`|SpawnActorFromClass` "/Game/Enemy/Projectile/BP_Projectile.BP_Projectile_C" (`KismetMathLibrary.MakeTransform` _returnvalue (`KismetMathLibrary.MakeRotator` _returnvalue_roll _returnvalue_pitch_2 _returnvalue_yaw)) "Undefined" "OverrideRootScale" null null))

(event `JumpAttack`
  ;[1 1 1] 점프 공격
  (`self.PlayAnimMontage` "/Game/Enemy/Anim/AM_JumpAttack.AM_JumpAttack"))

(event `self.LAttack.OnComponentBeginOverlap`
  (params (OverlappedComponent :type "PrimitiveComponent Object Reference") (OtherActor :type "Actor Object Reference") (OtherComp :type "PrimitiveComponent Object Reference") (OtherBodyIndex :type Integer) (bFromSweep :type Boolean) (SweepResult :type "HitResult Structure (by ref)"))
  ;[1 1 1] Comment
  (cast `/Game/Blueprints/BP_CCharacter` OtherActor)
  (set `self.bIsInL_AttackRange` true))

(event `self.LAttack.OnComponentEndOverlap`
  (params (OverlappedComponent :type "PrimitiveComponent Object Reference") (OtherActor :type "Actor Object Reference") (OtherComp :type "PrimitiveComponent Object Reference") (OtherBodyIndex :type Integer))
  ;[1 1 1] Comment
  (cast `/Game/Blueprints/BP_CCharacter` OtherActor)
  (set `self.bIsInL_AttackRange` false))

(event `self.CAttack.OnComponentBeginOverlap`
  (params (OverlappedComponent :type "PrimitiveComponent Object Reference") (OtherActor :type "Actor Object Reference") (OtherComp :type "PrimitiveComponent Object Reference") (OtherBodyIndex :type Integer) (bFromSweep :type Boolean) (SweepResult :type "HitResult Structure (by ref)"))
  ;[1 1 1] Comment
  (cast `/Game/Blueprints/BP_CCharacter` OtherActor)
  (set `self.bIsInC_AttackRange` true))

(event `self.CAttack.OnComponentEndOverlap`
  (params (OverlappedComponent :type "PrimitiveComponent Object Reference") (OtherActor :type "Actor Object Reference") (OtherComp :type "PrimitiveComponent Object Reference") (OtherBodyIndex :type Integer))
  ;[1 1 1] Comment
  (cast `/Game/Blueprints/BP_CCharacter` OtherActor)
  (set `self.bIsInC_AttackRange` false))

(fn `Death`
  ;[1 1 1] 죽음처리
  (`BrainComponent.StopLogic` (`AIController.BrainComponent` (`AIBlueprintHelperLibrary.GetAIController` self)) (`self.Reason`))
  (`PrimitiveComponent.SetCollisionEnabled` (`self.Mesh`) "NoCollision")
  (`PrimitiveComponent.SetCollisionEnabled` (`self.CapsuleComponent`) "NoCollision")
  (if (`KismetSystemLibrary.IsValid` (`self.CharacterMovement`))
    (`ActorComponent.K2_DestroyComponent` (`self.CharacterMovement`)))
  (return))

(fn `Update Walk Speed`
  (params (NewWalkSpeed :type "Float (double-precision)"))
  ;[1 1 1] 걷는 속도 조절
  (set `CharacterMovementComponent.MaxWalkSpeed` NewWalkSpeed (`self.CharacterMovement`)))

(fn `UserConstructionScript`)